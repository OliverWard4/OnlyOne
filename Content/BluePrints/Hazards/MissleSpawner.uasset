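; Hazard spawner that fires HomingMissle actors at the main character from the edges of a fixed rectangle.
; From BeginPlay it loops endlessly, picking one of four sides at random every half second and spawning a missile at a random point along that side on a fixed Y plane.
; Each missile receives its own box position as start and the character sprite's position at spawn time as its final target.
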(event `self.ReceiveBeginPlay`
  (bind _returnvalue (`KismetMathLibrary.RandomFloatInRange` -640.0 150.0))
  (bind _returnvalue_2 (`KismetMathLibrary.RandomFloatInRange` -480.0 270.0))
  (switch `int` (`KismetMathLibrary.RandomInteger` 4) :!label _label
    (:`0`
      (bind _returnvalue_3 (`|SpawnActorFromClass` "/Game/BluePrints/Hazards/HomingMissle.HomingMissle_C" (`KismetMathLibrary.MakeTransform` (`KismetMathLibrary.MakeVector` -640.0 -240.0 _returnvalue_2)) "Undefined" "MultiplyWithRoot" null null))
      (set `/Game/BluePrints/Hazards/HomingMissle.Start Location` (`SceneComponent.K2_GetComponentLocation` (`/Game/BluePrints/Hazards/DestructableObject.Box` _returnvalue_3)) _returnvalue_3)
      (set `/Game/BluePrints/Hazards/HomingMissle.Final Location` (`SceneComponent.K2_GetComponentLocation` (`PaperCharacter.Sprite` (`self.MainChar`))) _returnvalue_3))
    (:`1`
      (bind _returnvalue_4 (`|SpawnActorFromClass` "/Game/BluePrints/Hazards/HomingMissle.HomingMissle_C" (`KismetMathLibrary.MakeTransform` (`KismetMathLibrary.MakeVector` 150.0 -240.0 _returnvalue_2)) "Undefined" "MultiplyWithRoot" null null))
      (set `/Game/BluePrints/Hazards/HomingMissle.Start Location` (`SceneComponent.K2_GetComponentLocation` (`/Game/BluePrints/Hazards/DestructableObject.Box` _returnvalue_4)) _returnvalue_4)
      (set `/Game/BluePrints/Hazards/HomingMissle.Final Location` (`SceneComponent.K2_GetComponentLocation` (`PaperCharacter.Sprite` (`self.MainChar`))) _returnvalue_4))
    (:`2`
      (bind _returnvalue_5 (`|SpawnActorFromClass` "/Game/BluePrints/Hazards/HomingMissle.HomingMissle_C" (`KismetMathLibrary.MakeTransform` (`KismetMathLibrary.MakeVector` _returnvalue -240.0 270.0)) "Undefined" "MultiplyWithRoot" null null))
      (set `/Game/BluePrints/Hazards/HomingMissle.Start Location` (`SceneComponent.K2_GetComponentLocation` (`/Game/BluePrints/Hazards/DestructableObject.Box` _returnvalue_5)) _returnvalue_5)
      (set `/Game/BluePrints/Hazards/HomingMissle.Final Location` (`SceneComponent.K2_GetComponentLocation` (`PaperCharacter.Sprite` (`self.MainChar`))) _returnvalue_5))
    (:`3`
      (bind _returnvalue_6 (`|SpawnActorFromClass` "/Game/BluePrints/Hazards/HomingMissle.HomingMissle_C" (`KismetMathLibrary.MakeTransform` (`KismetMathLibrary.MakeVector` _returnvalue -240.0 -490.0)) "Undefined" "MultiplyWithRoot" null null))
      (set `/Game/BluePrints/Hazards/HomingMissle.Start Location` (`SceneComponent.K2_GetComponentLocation` (`/Game/BluePrints/Hazards/DestructableObject.Box` _returnvalue_6)) _returnvalue_6)
      (set `/Game/BluePrints/Hazards/HomingMissle.Final Location` (`SceneComponent.K2_GetComponentLocation` (`PaperCharacter.Sprite` (`self.MainChar`))) _returnvalue_6)))
  (`KismetSystemLibrary.Delay` 0.5)
  (goto _label))

(fn `UserConstructionScript`)