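; Homing missile hazard actor that moves a randomly tinted, semi-transparent Paper sprite along a straight path when play begins.
; A timed Delay loop advances the sprite by a constant fraction of the StartLocation-to-FinalLocation vector, divided by Speed, without sweeping or re-targeting.
; Once the step counter reaches its limit, the actor waits briefly and destroys itself.
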(event `self.ReceiveBeginPlay`
  (bind _index (`self.index`))
  (`PaperSpriteComponent.SetSpriteColor` (`self.PaperSprite`) (make `LinearColor` (`KismetMathLibrary.RandomFloatInRange` 0.0 1.0) (`KismetMathLibrary.RandomFloatInRange` 0.0 1.0) (`KismetMathLibrary.RandomFloatInRange` 0.0 1.0) 0.8))
  (if (< _index 60.0) :!label _label
    (`SceneComponent.K2_SetWorldLocation` (`self.PaperSprite`) (+ (`SceneComponent.K2_GetComponentLocation` (`self.PaperSprite`)) (/ (- (`self.Final Location`) (`self.Start Location`)) (`self.Speed`))) false false)
    (set `self.index` (+ _index 1.0))
    (`KismetSystemLibrary.Delay` 0.05)
    (goto _label)
    (else
      (`KismetSystemLibrary.Delay` 0.2)
      (`self.K2_DestroyActor`))))

(fn `UserConstructionScript`
  (`parent.UserConstructionScript`))