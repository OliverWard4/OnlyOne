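; GrowingLine is a hazard actor whose Paper sprite grows over about three seconds and then destroys itself.
; On BeginPlay, a looping Delay adds one sixtieth of NewScale to the sprite's world scale every 0.05 seconds.
; An Index counter ends the loop after 60 steps, so the total growth equals NewScale, and then calls DestroyActor.
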(event `self.ReceiveBeginPlay`
  (if (< (`self.index`) 60) :!label _label
    (`SceneComponent.SetWorldScale3D` (`self.PaperSprite`) (+ (`SceneComponent.K2_GetComponentScale` (`self.PaperSprite`)) (* (/ 1.0 60.0) (`self.New Scale`))))
    (set `self.index` (+ (`self.index`) 1.0))
    (`KismetSystemLibrary.Delay` 0.05)
    (goto _label)
    (else
      (`self.K2_DestroyActor`))))

(fn `UserConstructionScript`
  (`parent.UserConstructionScript`))